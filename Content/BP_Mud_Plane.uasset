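; BP_Mud_Plane is a mud surface actor that records left and right foot marks in the RT_Mud_Plane render target.
; On BeginPlay it creates a dynamic instance of the foot brush material and clears the render target to black.
; The Draw event takes 2D positions for both feet, sets them as brush vector parameters and draws the material into the target after each update.
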(event Custom|Draw
  (params (Right :type Vector%202D%20Structure) (Left :type Vector%202D%20Structure))
  (bind _brush_reff (Variables|Default|GetBrush%20Reff))
  (bind _brush_reff_2 (Variables|Default|GetBrush%20Reff))
  (Utilities|FlowControl|Sequence
    (:then_0
      (Rendering|Material|SetVectorParameterValue _brush_reff "right" (Math|Conversions|ToLinearColor(Vector) (Math|Conversions|ToVector(Vector2D) Right)) :!class /Script/Engine.MaterialInstanceDynamic)
      (Rendering|DrawMaterialtoRenderTarget "/Game/RT_Mud_Plane.RT_Mud_Plane" _brush_reff_2))
    (:then_1
      (Rendering|Material|SetVectorParameterValue _brush_reff "left" (Math|Conversions|ToLinearColor(Vector) (Math|Conversions|ToVector(Vector2D) Left)) :!class /Script/Engine.MaterialInstanceDynamic)
      (Rendering|DrawMaterialtoRenderTarget "/Game/RT_Mud_Plane.RT_Mud_Plane" _brush_reff_2))))

(event EventBeginPlay
  (bind _returnvalue (Rendering|Material|CreateDynamicMaterialInstance "/Game/M_Foot_brush_Inst.M_Foot_brush_Inst" "None" :!class /Script/Engine.KismetMaterialLibrary))
  (Variables|Default|SetBrush%20Reff _returnvalue)
  (Rendering|ClearRenderTarget2D "/Game/RT_Mud_Plane.RT_Mud_Plane"))

(event Collision|EventActorBeginOverlap
  (params (OtherActor :type Actor%20Object%20Reference)))

(event EventTick
  (params (DeltaSeconds :type Float%20%28single-precision%29)))

(fn ConstructionScript)